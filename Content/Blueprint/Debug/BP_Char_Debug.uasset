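; Debug character for testing movement and the Gameplay Ability System.
; Control-yaw-relative move input cancels click-to-move, which traces under the cursor and calls SimpleMoveToLocation; holding right mouse gates yaw look.
; BeginPlay grants a sample ability, initializes attributes from a DataTable, then tries activating the ability twice on delays, printing the second result.
; Tick prints attribute readouts labeled Strength and Physique.
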(event Input|EnhancedActionEvents|EnhancedInputActionIA_Move
  (params (ActionValue :type Vector%202D%20Structure) (ElapsedSeconds :type Float%20%28double-precision%29) (TriggeredSeconds :type Float%20%28double-precision%29) (InputAction :type Input%20Action%20Object%20Reference :default "/Game/Input/Action/IA_Move.IA_Move"))
  (bind _returnvalue (Pawn|GetControlRotation :!class /Script/Engine.Pawn))
  (Pawn|Input|AddMovementInput (Math|Vector|GetRightVector (Math|Rotator|MakeRotator (.roll _returnvalue) 0.0 (.yaw _returnvalue))) (.x ActionValue) false)
  (Pawn|Input|AddMovementInput (Math|Vector|GetForwardVector (Math|Rotator|MakeRotator 0.0 0.0 (.yaw (Pawn|GetControlRotation :!class /Script/Engine.Pawn)))) (.y ActionValue) false)
  (AI|Navigation|StopMovement (Pawn|GetController)))

(event Input|EnhancedActionEvents|EnhancedInputActionIA_Look
  (params (ActionValue :type Float%20%28double-precision%29) (ElapsedSeconds :type Float%20%28double-precision%29) (TriggeredSeconds :type Float%20%28double-precision%29) (InputAction :type Input%20Action%20Object%20Reference :default "/Game/Input/Action/IA_Look.IA_Look"))
  (Utilities|FlowControl|Gate true
    (:Exit
      (Pawn|Input|AddControllerYawInput ActionValue))))

(event Input|EnhancedActionEvents|EnhancedInputActionIA_Move_Mouse
  (params (ActionValue :type Boolean) (ElapsedSeconds :type Float%20%28double-precision%29) (TriggeredSeconds :type Float%20%28double-precision%29) (InputAction :type Input%20Action%20Object%20Reference :default "/Game/Input/Action/IA_Move_Mouse.IA_Move_Mouse"))
  (bind _returnvalue (Game|GetPlayerController 0))
  (bind (_worldlocation _worlddirection) (Game|Player|ConvertMouseLocationToWorldSpace _returnvalue))
  (:Triggered
    (bind _outhit (Collision|LineTraceByChannel _worldlocation (+ _worldlocation (* _worlddirection 1.92e+04)) "TraceTypeQuery1" false 0 "ForOneFrame" :!label _label))
    (AI|Navigation|SimpleMovetoLocation (Pawn|GetController) (.Location (Collision|BreakHitResult _outhit))))
  (:Started
    (goto _label))
  (:Ongoing
    (goto _label)))

(event EventBeginPlay
  (Utilities|FlowControl|Delay 0.5)
  (GameplayAbilities|GiveAbility (Variables|Default|GetAbilitySystem) "/Game/DataAsset/AbilityAsset/GA_SampleAbility.GA_SampleAbility_C" 1 -1)
  (Class|TireflyAbilitySystemComponent|InitAttributeSetfromDataTableRow (Variables|Default|GetAbilitySystem) "/Script/AsuraX.AsuraAttributeSet" "/Game/DataTable/Attribute/Sample/DT_AttributeSample.DT_AttributeSample" "1" false)
  (Utilities|FlowControl|Delay 1.0)
  (Abilities|TryActivateAbilitybyClass (Variables|Default|GetAbilitySystem) "/Game/DataAsset/AbilityAsset/GA_SampleAbility.GA_SampleAbility_C" true)
  (Utilities|FlowControl|Delay 5.5)
  (bind _returnvalue (Abilities|TryActivateAbilitybyClass (Variables|Default|GetAbilitySystem) "/Game/DataAsset/AbilityAsset/GA_SampleAbility.GA_SampleAbility_C" true))
  (Development|PrintString (Utilities|String|ToString(Boolean) _returnvalue) true false "(R=0.000000,G=0.660000,B=1.000000,A=1.000000)" 5.0))

(event EventTick
  (params (DeltaSeconds :type Float%20%28single-precision%29))
  (Development|PrintString (Utilities|String|Append "Strength" "///" (Utilities|String|ToString(Float) (.ReturnValue (Ability|Attribute|GetFloatAttribute self "(AttributeName=\"Strength\",Attribute=/Script/AsuraX.AsuraAttributeSet:Strength,AttributeOwner=\"/Script/CoreUObject.Class'/Script/AsuraX.AsuraAttributeSet'\")")))) true false "(R=0.000000,G=0.660000,B=1.000000,A=1.000000)" 0.0)
  (Development|PrintString (Utilities|String|Append "Physique" "///" (Utilities|String|ToString(Float) (.ReturnValue (Ability|Attribute|GetFloatAttribute self "(AttributeName=\"Physique\",Attribute=/Script/AsuraX.AsuraAttributeSet:Physique,AttributeOwner=\"/Script/CoreUObject.Class'/Script/AsuraX.AsuraAttributeSet'\")")))) true false "(R=0.000000,G=0.660000,B=1.000000,A=1.000000)" 0.0))

(event Input|MouseEvents|RightMouseButton
  (params (Key :type Key%20Structure :default "None"))
  (:Pressed
    (Utilities|FlowControl|Gate true) ; enters at Open
  )
  (:Released
    (Utilities|FlowControl|Gate true) ; enters at Close
  ))

(fn ConstructionScript)