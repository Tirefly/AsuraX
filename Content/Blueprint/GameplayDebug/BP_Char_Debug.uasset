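; Debug player character Blueprint for testing template combat abilities with sample data.
; Shortly after BeginPlay it initializes attributes from a sample DataTable row, binds a Tirefly gameplay input config, and grants template light, heavy and offset GAS abilities.
; Enhanced Input drives camera-relative movement and look.
; Attack inputs, on both Started and Triggered, are forwarded as gameplay-tagged StateTree events rather than activating abilities directly.
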(event EventBeginPlay
  (Utilities|FlowControl|Delay 0.5)
  (Class|TireflyAbilitySystemComponent|InitAttributeSetfromDataTableRow (Variables|Default|GetAbilitySystem) "/Script/AsuraX.AsuraAttributeSet" "/Game/DataTable/Attribute/Sample/DT_AttributeSample.DT_AttributeSample" "1" false)
  (Class|TireflyGameplayInputComponent|BindGameplayInputConfig (Variables|Default|GetTireflyGameplayInput) "/Game/Input/GameplayInputConfig_Sample.GameplayInputConfig_Sample")
  (GameplayAbilities|GiveAbility (Variables|Default|GetAbilitySystem) "/Game/Blueprint/AbilitySystem/Abilities/Template/GA_Template_LightAttack1.GA_Template_LightAttack1_C" 0 -1)
  (GameplayAbilities|GiveAbility (Variables|Default|GetAbilitySystem) "/Game/Blueprint/AbilitySystem/Abilities/Template/GA_Template_LightAttack2.GA_Template_LightAttack2_C" 0 -1)
  (GameplayAbilities|GiveAbility (Variables|Default|GetAbilitySystem) "/Game/Blueprint/AbilitySystem/Abilities/Template/GA_Template_LightAttack3.GA_Template_LightAttack3_C" 0 -1)
  (GameplayAbilities|GiveAbility (Variables|Default|GetAbilitySystem) "/Game/Blueprint/AbilitySystem/Abilities/Template/GA_Template_HeavyAttack1.GA_Template_HeavyAttack1_C" 0 -1)
  (GameplayAbilities|GiveAbility (Variables|Default|GetAbilitySystem) "/Game/Blueprint/AbilitySystem/Abilities/Template/GA_Template_HeavyAttack2.GA_Template_HeavyAttack2_C" 0 -1)
  (GameplayAbilities|GiveAbility (Variables|Default|GetAbilitySystem) "/Game/Blueprint/AbilitySystem/Abilities/Template/GA_Template_HeavyAttack3.GA_Template_HeavyAttack3_C" 0 -1)
  (GameplayAbilities|GiveAbility (Variables|Default|GetAbilitySystem) "/Game/Blueprint/AbilitySystem/Abilities/Template/GA_Template_HeavyAttack4.GA_Template_HeavyAttack4_C" 0 -1)
  (GameplayAbilities|GiveAbility (Variables|Default|GetAbilitySystem) "/Game/Blueprint/AbilitySystem/Abilities/Template/GA_Template_Offset.GA_Template_Offset_C" 0 -1))

(event EventTick
  (params (DeltaSeconds :type Float%20%28single-precision%29)))

(event Input|EnhancedActionEvents|EnhancedInputActionIA_Move
  (params (ActionValue :type Vector%202D%20Structure) (ElapsedSeconds :type Float%20%28double-precision%29) (TriggeredSeconds :type Float%20%28double-precision%29) (InputAction :type Input%20Action%20Object%20Reference :default "/Game/Input/Action/IA_Move.IA_Move"))
  (bind _returnvalue (Pawn|GetControlRotation :!class /Script/Engine.Pawn))
  (Pawn|Input|AddMovementInput (Math|Vector|GetRightVector (Math|Rotator|MakeRotator (.roll _returnvalue) 0.0 (.yaw _returnvalue))) (.x ActionValue) false)
  (Pawn|Input|AddMovementInput (Math|Vector|GetForwardVector (Math|Rotator|MakeRotator 0.0 0.0 (.yaw (Pawn|GetControlRotation :!class /Script/Engine.Pawn)))) (.y ActionValue) false))

(event Input|EnhancedActionEvents|EnhancedInputActionIA_Look
  (params (ActionValue :type Vector%202D%20Structure) (ElapsedSeconds :type Float%20%28double-precision%29) (TriggeredSeconds :type Float%20%28double-precision%29) (InputAction :type Input%20Action%20Object%20Reference :default "/Game/Input/Action/IA_Look.IA_Look"))
  (Pawn|Input|AddControllerYawInput (.x ActionValue))
  (Pawn|Input|AddControllerPitchInput (.y ActionValue)))

(event Input|EnhancedActionEvents|EnhancedInputActionIA_LightAttack
  (params (ActionValue :type Boolean) (ElapsedSeconds :type Float%20%28double-precision%29) (TriggeredSeconds :type Float%20%28double-precision%29) (InputAction :type Tirefly%20Input%20Action%20Object%20Reference :default "/Game/Input/Action/IA_LightAttack.IA_LightAttack"))
  (:Triggered
    (Gameplay|StateTree|SendStateTreeEvent (Variables|Default|GetStateTree) (Utilities|Struct|MakeStateTreeEvent "(TagName=\"InputAction.LightAttack\")") :!class /Script/GameplayStateTreeModule.StateTreeComponent :!label _label))
  (:Started
    (goto _label)))

(event Input|EnhancedActionEvents|EnhancedInputActionIA_HeavyAttack
  (params (ActionValue :type Boolean) (ElapsedSeconds :type Float%20%28double-precision%29) (TriggeredSeconds :type Float%20%28double-precision%29) (InputAction :type Tirefly%20Input%20Action%20Object%20Reference :default "/Game/Input/Action/IA_HeavyAttack.IA_HeavyAttack"))
  (:Triggered
    (Gameplay|StateTree|SendStateTreeEvent (Variables|Default|GetStateTree) (Utilities|Struct|MakeStateTreeEvent "(TagName=\"InputAction.HeavyAttack\")") :!class /Script/GameplayStateTreeModule.StateTreeComponent :!label _label))
  (:Started
    (goto _label)))

(event Input|EnhancedActionEvents|EnhancedInputActionIA_SpecialAttack
  (params (ActionValue :type Boolean) (ElapsedSeconds :type Float%20%28double-precision%29) (TriggeredSeconds :type Float%20%28double-precision%29) (InputAction :type Tirefly%20Input%20Action%20Object%20Reference :default "/Game/Input/Action/IA_SpecialAttack.IA_SpecialAttack"))
  (:Triggered
    (Gameplay|StateTree|SendStateTreeEvent (Variables|Default|GetStateTree) (Utilities|Struct|MakeStateTreeEvent "(TagName=\"InputAction.SpecialAttack\")") :!class /Script/GameplayStateTreeModule.StateTreeComponent :!label _label))
  (:Started
    (goto _label)))

(fn ConstructionScript)